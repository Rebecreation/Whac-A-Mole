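; Spawner actor that grows one random vegetable at a time under the control of a vegetable manager.
; On activation it picks a Veggies entry, sets its mesh and dynamic material, then waits a random dormant time.
; Tick scales the actor up to full size, then calls TryPick after a random autopick delay.
; Picking notifies the manager and deactivates the spawner; disabling pauses Tick logic and flags the material.
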(event EventBeginPlay
  (Transformation|SetActorScale3D "0, 0, 0"))

(event Collision|EventActorBeginOverlap
  (params (OtherActor :type Actor%20Object%20Reference)))

(event EventTick
  (params (DeltaSeconds :type Float%20%28single-precision%29))
  (bind _returnvalue (Transformation|GetActorScale3D))
  (bind _currentveggieindex (Variables|Default|GetCurrentVeggieIndex))
  (bind _veggies (Variables|Default|GetVeggies))
  (bind _veggies_2 (Variables|Default|GetVeggies))
  (bind _currentveggieindex_2 (Variables|Default|GetCurrentVeggieIndex))
  (bind _output (Utilities|Array|Get(acopy) _veggies_2 _currentveggieindex))
  (bind _output_2 (Utilities|Array|Get(acopy) _veggies _currentveggieindex_2))
  (bind _growspeed (Utilities|Struct|BreakWmVeggieData _output))
  (bind _maxscale (Utilities|Struct|BreakWmVeggieData _output_2))
  (bind _returnvalue_2 (* _growspeed DeltaSeconds))
  (bind _returnvalue_3 (+ _returnvalue _returnvalue_2))
  (bind (_x _y _z) (Math|Vector|BreakVector _returnvalue_3))
  (bind _returnvalue_4 (Math|Float|Clamp(Float) _x 0.0 _maxscale))
  (if (Variables|Default|GetIsActive)
    (if (not (Variables|Default|GetbIsDisabled))
      (if (!= _currentveggieindex_2 -1)
        (if (>= (Utilities|Time|GetGameTimeinSeconds) (Variables|Default|GetDormantGameTime))
          (Transformation|SetActorScale3D (Math|Vector|MakeVector _returnvalue_4 (Math|Float|Clamp(Float) _y 0.0 _maxscale) (Math|Float|Clamp(Float) _z 0.0 _maxscale)))
          (if (Math|Float|NearlyEqual(Float) _returnvalue_4 _maxscale 1e-06)
            (if (Variables|Default|GetisGrown)
              (if (>= (Utilities|Time|GetGameTimeinSeconds) (Variables|Default|GetgrownAutopickTime))
                (Class|WmVeggieSpawner|TryPick))
              (else
                (CallFunction|OnGrownComplete)))))))))

(event EventOnPicked
  (Default|OnInactiveEvent (Variables|Default|GetManager) self)
  (CallFunction|SetSpawnerActive false))

(event EventOnDisabled
  (Variables|Default|SetbIsDisabled true)
  (Rendering|Material|SetScalarParameterValue (Variables|Default|GetMaterial) "IsDisabled" 1.0 :!class /Script/Engine.MaterialInstanceDynamic))

(event EventOnReenable
  (Variables|Default|SetbIsDisabled false)
  (Rendering|Material|SetScalarParameterValue (Variables|Default|GetMaterial) "IsDisabled" 0.0 :!class /Script/Engine.MaterialInstanceDynamic))

(fn ConstructionScript)

(fn SetSpawnerActive
  (params (Is%20Active :type Boolean) (Veggie%20Manager :type BP%20Vegetable%20Manager%20Object%20Reference))
  (bind _veggiemesh (Variables|Default|GetVeggieMesh))
  (bind _output_get (Variables|Default|SetIsActive Is%20Active))
  (Variables|Default|SetManager Veggie%20Manager)
  (if _output_get
    (bind _output_get_2 (Variables|Default|SetCurrentVeggieIndex (Math|Random|RandomIntegerinRange 0 (- (Utilities|Array|Length (Variables|Default|GetVeggies)) 1))))
    (Components|StaticMesh|SetStaticMesh (Variables|Default|GetVeggieMesh) (.VeggieMesh (Utilities|Struct|BreakWmVeggieData (Utilities|Array|Get(acopy) (Variables|Default|GetVeggies) _output_get_2))))
    (Rendering|SetVisibility (Variables|Default|GetVeggieMesh) true true)
    (Transformation|SetActorScale3D "0, 0, 0")
    (bind _returnvalue (Rendering|Material|CreateDynamicMaterialInstance _veggiemesh 0 (Rendering|Material|GetMaterial _veggiemesh 0) "None" :!class /Script/Engine.PrimitiveComponent))
    (bind _output_get_3 (Variables|Default|SetMaterial _returnvalue))
    (Rendering|Material|SetMaterial _veggiemesh 0 _output_get_3)
    (Variables|Default|SetisGrown false)
    (Variables|Default|SetDormantGameTime (+ (Utilities|Time|GetGameTimeinSeconds) (Math|Random|RandomFloatinRange (.X (Math|Vector2D|BreakVector2D (.DormantTime (Utilities|Struct|BreakWmVeggieData (Utilities|Array|Get(acopy) (Variables|Default|GetVeggies) _output_get_2))))) (.Y (Math|Vector2D|BreakVector2D (.DormantTime (Utilities|Struct|BreakWmVeggieData (Utilities|Array|Get(acopy) (Variables|Default|GetVeggies) _output_get_2))))))))))

(fn OnGrownComplete
  (bind _currentveggieindex (Variables|Default|GetCurrentVeggieIndex))
  (bind _veggies (Variables|Default|GetVeggies))
  (bind _output (Utilities|Array|Get(acopy) _veggies _currentveggieindex))
  (bind _autopicktime (Utilities|Struct|BreakWmVeggieData _output))
  (bind (_x _y) (Math|Vector2D|BreakVector2D _autopicktime))
  (Variables|Default|SetisGrown true)
  (Variables|Default|SetgrownAutopickTime (+ (Utilities|Time|GetGameTimeinSeconds) (Math|Random|RandomFloatinRange _x _y))))