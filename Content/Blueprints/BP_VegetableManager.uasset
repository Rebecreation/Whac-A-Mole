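; BP_VegetableManager controls which vegetable spawners are active in the level.
; On BeginPlay it activates several random inactive spawners from its soft-referenced VeggieSpawner list and binds to their OnInactive events.
; When one fires, it unbinds and activates another random inactive spawner, excluding the one that just finished.
; Replacement spawners are not bound to OnInactive here, so only the initial picks trigger a replacement through this manager.
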(event Custom|OnInactive_Event
  (params (Spawner :type BP%20Vegetable%20Spawner%20Object%20Reference))
  (EventDispatchers|UnbindEventfromOnInactive Spawner (delegate Custom|OnInactive_Event))
  (bind _spawner (CallFunction|GetRandomInactiveSpawner Spawner))
  (Utilities|IsValid _spawner
    (:Is%20Valid
      (Default|SetSpawnerActive _spawner true self))))

(event EventBeginPlay
  (for _index (range 0 3)
    (bind _spawner (CallFunction|GetRandomInactiveSpawner))
    (Utilities|IsValid _spawner
      (:Is%20Valid
        (Default|SetSpawnerActive _spawner true self)
        (EventDispatchers|AssignOnInactive _spawner (delegate Custom|OnInactive_Event))))))

(event Collision|EventActorBeginOverlap
  (params (OtherActor :type Actor%20Object%20Reference)))

(event EventTick
  (params (DeltaSeconds :type Float%20%28single-precision%29)))

(fn ConstructionScript)

(fn GetRandomInactiveSpawner
  (params (SpawnerToExclude :type BP%20Vegetable%20Spawner%20Object%20Reference))
  (bind _resultindeces (LocalVariables|GetresultIndeces))
  (bind _outitem (Utilities|Array|Random _resultindeces))
  (for (_array_element _array_index) (Variables|Default|GetVeggieSpawner)
    (if (Utilities|IsValidSoftObjectReference _array_element)
      (if (not (Variables|/Script/WhacAMole.WmVeggieSpawner|GetbIsActive (Utilities|ResolveSoftReference _array_element)))
        (if (not (== (Utilities|ResolveSoftReference _array_element) SpawnerToExclude))
          (Utilities|Array|Add (LocalVariables|GetresultIndeces) _array_index)))))
  (return _outitem (Utilities|ResolveSoftReference (Utilities|Array|Get(acopy) (Variables|Default|GetVeggieSpawner) _outitem))))